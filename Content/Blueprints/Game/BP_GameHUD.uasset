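; BP_GameHUD handles pausing and resuming the game through a pause menu widget.
; OnPause acts as a toggle: it pauses, creates and stores a WBP_PauseMenu, shows the cursor and switches input to Game and UI, or resumes if already paused.
; OnPauseContinue unpauses, removes the given menu if valid, restores game-only input and hides the cursor.
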(event `OnPauseContinue`
  (params (PauseMenu :type "/Game/UI/PauseMenu/WBP_PauseMenu Object Reference"))
  (bind _returnvalue (`GameplayStatics.GetPlayerController` 0))
  (`GameplayStatics.SetGamePaused` false)
  (`/Engine/EditorBlueprintResources/StandardMacros.IsValid` PauseMenu
    (:`Is Valid`
      (`Widget.RemoveFromParent` PauseMenu))
    (:`Is Not Valid`
      _))
  (`WidgetBlueprintLibrary.SetInputMode_GameOnly` _returnvalue true)
  (set `PlayerController.bShowMouseCursor` false _returnvalue))

(event `OnPause`
  (bind _returnvalue (`GameplayStatics.GetPlayerController` 0))
  (if (`GameplayStatics.IsGamePaused`)
    (`self.OnPauseContinue` (`self.Pause`))
    (else
      (`GameplayStatics.SetGamePaused` true)
      (bind _returnvalue_2 (`|CreateWidget` "/Game/UI/PauseMenu/WBP_PauseMenu.WBP_PauseMenu_C"))
      (`UserWidget.AddToViewport` _returnvalue_2 0)
      (set `self.Pause` _returnvalue_2)
      (set `PlayerController.bShowMouseCursor` true _returnvalue)
      (`WidgetBlueprintLibrary.SetInputMode_GameAndUIEx` _returnvalue _returnvalue_2))))

(fn `UserConstructionScript`)