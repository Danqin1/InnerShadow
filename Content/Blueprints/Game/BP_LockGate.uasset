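; BP_LockGate is a two-leaf gate that swings open and closed.
; Open and Close events check and set an IsOpen flag, then each plays its own timeline to lerp GateLeft and GateRight between their closed and open relative rotations.
; On BeginPlay, StartOpen selects which event runs, so the timeline only plays if IsOpen differs from that state.
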(event `self.ReceiveBeginPlay`
  (if (`self.startOpen`)
    (`self.Open`)
    (else
      (`self.Close`))))

(event `self.Open`
  (if (not (`self.isOpen`))
    (set `self.isOpen` true)
    (bind (_direction _newtrack_0) (`Timeline|Timeline` :!via `PlayFromStart`)
      (:`Update`
        (`SceneComponent.K2_SetRelativeRotation` (`self.GateLeft`) (`KismetMathLibrary.RLerp` (`self.leftCloseRot`) (`self.leftOpenRot`) _newtrack_0) false false)
        (`SceneComponent.K2_SetRelativeRotation` (`self.GateRight`) (`KismetMathLibrary.RLerp` (`self.rightCloseRot`) (`self.rightOpenRot`) _newtrack_0) false false)))))

(event `self.Close`
  (if (`self.isOpen`)
    (set `self.isOpen` false)
    (bind (_direction _newtrack_0) (`Timeline|Timeline_0` :!via `PlayFromStart`)
      (:`Update`
        (`SceneComponent.K2_SetRelativeRotation` (`self.GateLeft`) (`KismetMathLibrary.RLerp` (`self.leftOpenRot`) (`self.leftCloseRot`) _newtrack_0) false false)
        (`SceneComponent.K2_SetRelativeRotation` (`self.GateRight`) (`KismetMathLibrary.RLerp` (`self.rightOpenRot`) (`self.rightCloseRot`) _newtrack_0) false false)))))

(fn `UserConstructionScript`)