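; BP_TimedCutscene is an actor that automatically plays a level sequence cutscene a set delay after BeginPlay.
; It puts the player's BP_TopDownCharacter into the Cutscene state, assigns the Sequence to its SequenceActor and plays it.
; A binding to the sequence player's OnFinished is meant to restore the character to Nothing and call OnCutsceneEnd, an empty function.
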(event `self.ReceiveBeginPlay`
  (bind _sequenceactor (`self.SequenceActor`))
  (bind _sequenceplayer (`LevelSequenceActor.SequencePlayer` _sequenceactor))
  (`KismetSystemLibrary.Delay` (`self.Delay`))
  (bind _asbp_top_down_character (cast `/Game/Blueprints/Player/BP_TopDownCharacter` (`GameplayStatics.GetPlayerCharacter` 0)))
  (set `self.As BP Top Down Character` _asbp_top_down_character)
  (`RPGCharacter.SetState` _asbp_top_down_character "Cutscene")
  (`LevelSequenceActor.SetSequence` _sequenceactor (`self.Sequence`))
  (`MovieSceneSequencePlayer.Play` _sequenceplayer)
  (add `MovieSceneSequencePlayer.OnFinished` _sequenceplayer (`|CreateDelegate` :!event `OnCutsceneFinished`)))

(event `OnCutsceneFinished`
  (bind _as_bp_top_down_character (`self.As BP Top Down Character`)
    (:`then`
      (`RPGCharacter.SetState` _as_bp_top_down_character "Nothing"))
    (:`else`
      _))
  (`self.OnCutsceneEnd`))

(fn `OnCutsceneEnd`)

(fn `UserConstructionScript`)