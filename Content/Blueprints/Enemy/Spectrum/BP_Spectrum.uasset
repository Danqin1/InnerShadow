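; BP_Spectrum is an enemy with an area attack targeted at the player's position, with lightning effects.
; On BeginPlay its SkeletalMesh follows the pose of the main Mesh.
; SpawnIndicator spawns an attack indicator at the controlled pawn's transform and plays a lightning effect on itself.
; OnAttackAnimEnd sphere-traces for pawns at the indicator's location, applying Combat's current damage once per actor through IDamageable.
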(event `self.ReceiveBeginPlay`
  (`SkinnedMeshComponent.SetLeaderPoseComponent` (`self.SkeletalMesh`) (`self.Mesh`) false false))

(fn `OnAttackAnimEnd`
  (locals (AtkLoc :type "Vector Structure" :default (0.0 0.0 0.0)) (HittedActors :type "Array of Actor Object Reference"))
  (bind _atkindicator (`self.AtkIndicator`)
    (:`then`
      (bind _output_get (set `local.AtkLoc` (`self.K2_GetActorLocation` _atkindicator))))
    (:`else`
      _))
  (bind _outhits (`KismetSystemLibrary.SphereTraceMultiForObjects` _output_get _output_get (`self.AttackRadius`) (`|MakeArray` "ObjectTypeQuery3" :!type "EObjectTypeQuery Enum")))
  (set `local.HittedActors` (`|MakeArray`))
  (for _array_element _outhits
    (bind (_bblockinghit _binitialoverlap _time _distance _location _impactpoint _normal _impactnormal _physmat _hitactor) (`GameplayStatics.BreakHitResult` _array_element))
    (if (`KismetSystemLibrary.DoesImplementInterface` _hitactor "/Script/TopDownRPG.IDamageable")
      (bind _returnvalue (message `IDamageable.CanDamage` _hitactor))
      (if (and _returnvalue (not (`KismetArrayLibrary.Array_Contains` (`local.HittedActors`) _hitactor)))
        (message `IDamageable.Damage` _hitactor (`EnemyCombatBase.CurrentDamage` (`self.Combat`)))
        (`KismetArrayLibrary.Array_Add` (`local.HittedActors`) _hitactor)))))

(fn `SpawnIndicator`
  (bind _returnvalue (`|SpawnActorFromClass` "/Game/Blueprints/Enemy/Spectrum/BP_SpectrumAtkEffect.BP_SpectrumAtkEffect_C" (`self.GetTransform` (`Controller.K2_GetPawn` (`GameplayStatics.GetPlayerController` 0))) "Undefined" "MultiplyWithRoot" null self))
  (bind _output_get (set `self.AtkIndicator` _returnvalue))
  (`/Game/Blueprints/Enemy/Spectrum/BP_SpectrumAtkEffect.OnStartAttack` _output_get 0.0)
  (`NiagaraFunctionLibrary.SpawnSystemAttached` "/Game/VFX/FX_Lighting_Start.FX_Lighting_Start" (`self.Mesh`) "None" (0.0 0.0 150.0) (struct) "KeepRelativeOffset" true))

(fn `UserConstructionScript`)