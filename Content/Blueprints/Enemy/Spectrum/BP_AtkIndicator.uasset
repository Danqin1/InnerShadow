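; Attack indicator for the Spectrum enemy that shows an attack's wind-up through a Niagara effect.
; Attack start stores the duration, resets the timer, activates Niagara and zeroes the "Charge" float parameter.
; Each update accumulates delta time and sends elapsed over full duration as Charge, via the reference from the component's GetAsset.
; Attack end deactivates the effect.
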(event `OnStartAttack`
  (params (AttackIndicatorDuration :type "Float (double-precision)"))
  (bind _niagara (`self.Niagara`))
  (set `self.AttackFullDuration` AttackIndicatorDuration)
  (bind _output_get (set `self.AttackCurrentDuration` 0.0))
  (`ActorComponent.Activate` _niagara true)
  (bind _output_get_2 (set `self.VFX` (`NiagaraComponent.GetAsset` _niagara)))
  (message `AudioParameterControllerInterface.SetFloatParameter` _output_get_2 "Charge" _output_get))

(event `OnUpdateAttack`
  (params (Delta :type "Float (double-precision)"))
  (bind _output_get (set `self.AttackCurrentDuration` (+ (`self.AttackCurrentDuration`) Delta)))
  (message `AudioParameterControllerInterface.SetFloatParameter` (`self.VFX`) "Charge" (/ _output_get (`self.AttackFullDuration`))))

(event `OnAttackEnd`
  (`ActorComponent.Deactivate` (`self.Niagara`)))

(fn `UserConstructionScript`)