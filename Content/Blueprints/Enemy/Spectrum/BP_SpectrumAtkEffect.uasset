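; Attack effect for the Spectrum enemy: a moving Niagara effect that damages the player.
; On attack start it activates the effect, turns once toward the player and clears its hit list.
; Each tick it moves straight forward and sphere-traces pawns, hitting damageable player actors once each with block-crushing hits.
; Attack end stops damage and destroys the actor after a delay; the charge-progress update is unconnected.
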(event `OnStartAttack`
  (params (AttackIndicatorDuration :type "Float (double-precision)"))
  (bind _niagara (`self.Niagara`))
  (set `self.AttackFullDuration` AttackIndicatorDuration)
  (bind _output_get (set `self.AttackCurrentDuration` 0.0))
  (`ActorComponent.Activate` _niagara true)
  (bind _output_get_2 (set `self.VFX` (`NiagaraComponent.GetAsset` _niagara)))
  (message `AudioParameterControllerInterface.SetFloatParameter` _output_get_2 "Charge" _output_get)
  (set `self.doesDamage` true)
  (`self.K2_SetActorRotation` (`KismetMathLibrary.FindLookAtRotation` (`self.K2_GetActorLocation`) (`self.K2_GetActorLocation` (`GameplayStatics.GetPlayerCharacter` 0))))
  (set `self.HittedActors` (`|MakeArray`)))

(event `self.ReceiveTick`
  (params (DeltaSeconds :type "Float (single-precision)"))
  (if (`self.doesDamage`)
    (`self.Move` DeltaSeconds)
    (`self.TraceDamage`)))

(event `OnUpdateAttack`
  (params (Delta :type "Float (double-precision)")))

(event `OnAttackEnd`
  (set `self.doesDamage` false)
  (`ActorComponent.Deactivate` (`self.Niagara`))
  (`KismetSystemLibrary.Delay` 2.0)
  (`self.K2_DestroyActor`))

(fn `Move`
  (params (A :type "Float (double-precision)"))
  (bind _returnvalue (`self.K2_GetActorLocation`))
  (`self.K2_SetActorLocation` (`KismetMathLibrary.VLerp` _returnvalue (+ _returnvalue (* (`KismetMathLibrary.Normal` (`self.GetActorForwardVector`)) 100.0)) (* A (`self.Speed`))) false true))

(fn `TraceDamage`
  (bind _returnvalue (`self.K2_GetActorLocation`))
  (bind _outhits (`KismetSystemLibrary.SphereTraceMultiForObjects` :`Start` _returnvalue :`End` _returnvalue :`Radius` (`self.AttackRadius`) :`ObjectTypes` (`|MakeArray` "ObjectTypeQuery3" :!type "EObjectTypeQuery Enum") :`DrawTime` 0.1))
  (for _array_element _outhits
    (bind (_bblockinghit _binitialoverlap _time _distance _location _impactpoint _normal _impactnormal _physmat _hitactor) (`GameplayStatics.BreakHitResult` _array_element))
    (bind _ascombat_interface (cast `CombatInterface` _hitactor))
    (cast `PlayerInterface` _hitactor)
    (bind _returnvalue_2 (`CombatInterface.CanDamage` _ascombat_interface))
    (if (and _returnvalue_2 (not (`KismetArrayLibrary.Array_Contains` (`self.HittedActors`) _hitactor)))
      (`CombatInterface.Hit` _ascombat_interface null _impactpoint (0.0 0.0 0.0) (`self.Damage`) true true null)
      (`KismetArrayLibrary.Array_Add` (`self.HittedActors`) _hitactor))))

(fn `UserConstructionScript`)