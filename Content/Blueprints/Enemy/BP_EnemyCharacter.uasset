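; Enemy character Blueprint that drives an attack indicator widget to show the progress of an attack.
; BeginPlay caches the WBP_AttackIndicator from its Widget component and hides it.
; OnStartAttack resets and shows the indicator, OnUpdateAttack accumulates delta time into a fill percent over the given duration, and OnAttackEnd collapses it.
; The graph holds only this display logic, with no attack or damage handling.
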(event `self.ReceiveBeginPlay`
  (bind _aswbp_attack_indicator (cast `/Game/UI/Enemy/WBP_AttackIndicator` (`WidgetComponent.GetWidget` (`self.Widget`))))
  (bind _output_get (set `self.As WBP Attack Indicator` _aswbp_attack_indicator))
  (`Widget.SetVisibility` _output_get "Collapsed"))

(event `OnStartAttack`
  (params (AttackIndicatorDuration :type "Float (double-precision)"))
  (bind _as_wbp_attack_indicator (`self.As WBP Attack Indicator`))
  (set `self.AttackFullDuration` AttackIndicatorDuration)
  (set `self.AttackCurrentDuration` 0.0)
  (`Widget.SetVisibility` _as_wbp_attack_indicator "SelfHitTestInvisible")
  (`/Game/UI/Enemy/WBP_AttackIndicator.SetPercent` _as_wbp_attack_indicator 0.0))

(event `OnUpdateAttack`
  (params (Delta :type "Float (double-precision)"))
  (bind _output_get (set `self.AttackCurrentDuration` (+ (`self.AttackCurrentDuration`) Delta)))
  (`/Game/UI/Enemy/WBP_AttackIndicator.SetPercent` (`self.As WBP Attack Indicator`) (/ _output_get (`self.AttackFullDuration`))))

(event `OnAttackEnd`
  (`Widget.SetVisibility` (`self.As WBP Attack Indicator`) "Collapsed"))

(fn `UserConstructionScript`)