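; Roar of Darkness ability effect: an area life drain that damages nearby enemies and heals the caster.
; On activation it plays an airborne montage, gathers enemies with a single sphere trace and feeds their positions to an attached Niagara system.
; While caster and VFX are valid, Tick updates those positions, triggers hit reactions and converts frame-scaled damage into caster HP.
; After one second it stops the montage and signals completion.
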(event `self.BP_Activate`
  (params (Caster :type "Character Object Reference"))
  (bind _enemies (`self.Enemies`))
  (bind _returnvalue (`self.K2_GetActorLocation` (`self.As BP Top Down Character`)))
  (bind _asbp_top_down_character (cast `/Game/Blueprints/Player/BP_TopDownCharacter` Caster))
  (`Character.PlayAnimMontage` _asbp_top_down_character "/Game/Characters/RPG/Animations/LightSword/Jump/AM_Airborne.AM_Airborne" 1.0 "None")
  (bind _output_get (set `self.As BP Top Down Character` _asbp_top_down_character))
  (bind _returnvalue_2 (`NiagaraFunctionLibrary.SpawnSystemAttached` "/Game/VFX/RoarOfDarkness/NS_RoarOfDarkness.NS_RoarOfDarkness" (`Actor.RootComponent` _output_get) "None" (0.0 0.0 0.0) (struct) "SnapToTarget" true false))
  (set `self.VFX` _returnvalue_2)
  (set `self.Enemies` (`|MakeArray`))
  (bind (_outhits _returnvalue_3) (`KismetSystemLibrary.SphereTraceMultiForObjects` _returnvalue _returnvalue (`self.Radius`) (`|MakeArray` "ObjectTypeQuery3" :!type "EObjectTypeQuery Enum") false (`|MakeArray` (`self.As BP Top Down Character`) :!type "Actor Object Reference") "ForDuration"))
  (if _returnvalue_3
    (for _array_element _outhits
      (bind (_bblockinghit _binitialoverlap _time _distance _location _impactpoint _normal _impactnormal _physmat _hitactor) (`GameplayStatics.BreakHitResult` _array_element))
      (cast `EnemyInterface` _hitactor)
      (if (not (`KismetArrayLibrary.Array_Contains` _enemies _hitactor))
        (`KismetArrayLibrary.Array_Add` _enemies _hitactor)
        (bind _returnvalue_4 (`self.K2_GetActorLocation` _hitactor))
        (`KismetArrayLibrary.Array_Add` (`self.Positions`) _returnvalue_4)
        (`KismetSystemLibrary.PrintString` (`KismetStringLibrary.Concat_StrStr` "Enemy loc: " (`KismetStringLibrary.Conv_VectorToString` _returnvalue_4))))))
  (`NiagaraDataInterfaceArrayFunctionLibrary.SetNiagaraArrayPosition` (`self.VFX`) "Positions" (`self.Positions`))
  (`ActorComponent.Activate` (`self.VFX`) true)
  (`KismetSystemLibrary.Delay` 1.0)
  (`Character.StopAnimMontage` (`self.As BP Top Down Character`) "/Game/Characters/RPG/Animations/LightSword/Jump/AM_Airborne.AM_Airborne")
  (`self.OnEffectFinished` true))

(event `self.ReceiveTick`
  (params (DeltaSeconds :type "Float (single-precision)"))
  (bind _returnvalue (* (`self.Damage`) DeltaSeconds))
  (if (and (`KismetSystemLibrary.IsValid` (`self.As BP Top Down Character`)) (`KismetSystemLibrary.IsValid` (`self.VFX`)))
    (`KismetArrayLibrary.Array_Clear` (`self.Positions`))
    (for _array_element (`self.Enemies`)
      (`KismetArrayLibrary.Array_Add` (`self.Positions`) (+ (`self.K2_GetActorLocation` _array_element) (0.0 0.0 80.0)))
      (bind _asenemy_interface (cast `EnemyInterface` _array_element))
      (`EnemyInterface.OnHit` _asenemy_interface null (0.0 0.0 0.0) (0.0 0.0 0.0))
      (`EnemyInterface.OnSkillReaction` _asenemy_interface (`self.NPCReaction`))
      (bind _asdamageable_interface (cast `DamageableInterface` _array_element))
      (`DamageableInterface.Damage` _asdamageable_interface _returnvalue)
      (`PlayerStatsComponent.AddHP` (`RPGCharacter.PlayerStatsComponent` (`self.As BP Top Down Character`)) _returnvalue))
    (`NiagaraDataInterfaceArrayFunctionLibrary.SetNiagaraArrayPosition` (`self.VFX`) "Positions" (`self.Positions`))))

(fn `UserConstructionScript`)