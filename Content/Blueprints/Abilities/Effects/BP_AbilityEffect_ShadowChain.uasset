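; Ability effect actor named ShadowChain that performs an ice attack, freezing and damaging enemies around and ahead of the top-down character caster.
; Activate attaches Niagara VFX, then GetTargets merges a head-height cone trace with a close sphere trace, proceeding only on a cone hit.
; Targets are frozen through EnemyInterface, hit through CombatInterface and given ice materials.
; After timed delays it signals completion, unfreezes targets, restores only material slot 0 and destroys itself.
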(event `self.BP_Activate`
  (params (Caster :type "Character Object Reference"))
  (bind _asbp_top_down_character (cast `/Game/Blueprints/Player/BP_TopDownCharacter` Caster))
  (bind _output_get (set `self.As BP Top Down Character` _asbp_top_down_character))
  (bind _returnvalue (`NiagaraFunctionLibrary.SpawnSystemAttached` "/Game/VFX/NS_Ice_Attack.NS_Ice_Attack" (`Actor.RootComponent` _output_get) "None" (0.0 0.0 0.0) (struct) "SnapToTarget" true))
  (set `self.VFX` _returnvalue)
  (bind _returnvalue_location (`KismetMathLibrary.BreakTransform` (`SceneComponent.GetSocketTransform` (`Character.Mesh` _output_get) "head" "RTS_Actor")))
  (`NiagaraComponent.SetVariableVec3` _returnvalue "Position" _returnvalue_location)
  (`ActorComponent.Activate` _returnvalue true)
  (bind (_returnvalue_2 _outhits) (`self.GetTargets`))
  (`KismetSystemLibrary.Delay` 0.2)
  (if _returnvalue_2
    (for _array_element _outhits
      (bind (_bblockinghit _binitialoverlap _time _distance _location _impactpoint _normal _impactnormal _physmat _hitactor) (`GameplayStatics.BreakHitResult` _array_element))
      (bind _asenemy_interface (cast `EnemyInterface` _hitactor))
      (`KismetArrayLibrary.Array_Add` (`self.Hitted`) _hitactor)
      (bind _returnvalue_3 (`self.GetComponentByClass` _hitactor "/Script/Engine.SkeletalMeshComponent"))
      (`BlueprintMapLibrary.Map_Add` (`self.DefaultMaterials`) _hitactor (`PrimitiveComponent.GetMaterial` _returnvalue_3 0))
      (`EnemyInterface.Freeze` _asenemy_interface true)
      (bind _ascombat_interface (cast `CombatInterface` _hitactor))
      (`CombatInterface.Hit` _ascombat_interface null (0.0 0.0 0.0) (0.0 0.0 0.0) (`self.Damage`) false true null)
      (`NiagaraFunctionLibrary.SpawnSystemAtLocation` "/Game/VFX/BreathOfIce/NS_FrozenStart.NS_FrozenStart" (`self.K2_GetActorLocation` _hitactor))
      (`PrimitiveComponent.SetMaterial` _returnvalue_3 0 "/Game/Materials/Ice/MI_Ice.MI_Ice")
      (`PrimitiveComponent.SetMaterial` _returnvalue_3 1 "/Game/Materials/Ice/MI_Ice.MI_Ice")))
  (`KismetSystemLibrary.Delay` (`self.EffectDuration`))
  (`self.OnEffectFinished` false)
  (`KismetSystemLibrary.Delay` (`self.FrostedDuration`))
  (for _array_element_2 (`self.Hitted`)
    (`/Engine/EditorBlueprintResources/StandardMacros.IsValid` _array_element_2
      (:`Is Valid`
        (bind _asenemy_interface_2 (cast `EnemyInterface` _array_element_2))
        (`EnemyInterface.Freeze` _asenemy_interface_2 false)
        (bind (_value _returnvalue_4) (`BlueprintMapLibrary.Map_Find` (`self.DefaultMaterials`) _array_element_2))
        (if _returnvalue_4
          (`PrimitiveComponent.SetMaterial` (`self.GetComponentByClass` _array_element_2 "/Script/Engine.SkeletalMeshComponent") 0 _value)))))
  (`self.K2_DestroyActor`))

(fn `GetTargets`
  (returns (ReturnValue :type Boolean) (OutHits :type "Array of HitResult Structure"))
  (locals (Targets :type "Array of HitResult Structure"))
  (bind _returnvalue (`self.K2_GetActorLocation` (`self.As BP Top Down Character`)))
  (bind _array (`|MakeArray` (`self.As BP Top Down Character`) :!type "Actor Object Reference"))
  (bind _mesh (`Character.Mesh` (`self.As BP Top Down Character`)))
  (bind (_returnvalue_roll _returnvalue_pitch _returnvalue_yaw) (`KismetMathLibrary.BreakRotator` (`SceneComponent.GetSocketRotation` _mesh "None")))
  (bind (_outhits _returnvalue_2) (`RPGFunctionsLibrary.ConeTraceMulti` (`SceneComponent.GetSocketLocation` _mesh "head") (`KismetMathLibrary.MakeRotator` _returnvalue_roll _returnvalue_pitch (+ _returnvalue_yaw 90.0)) (`self.Radius`) 30.0 "TraceTypeQuery3" false _array "ForDuration" (struct :`R` 0.412908 :`G` 1.0 :`B` 0.045183 :`A` 1.0) (struct :`R` 1.0 :`B` 0.114695 :`A` 1.0) 5.0))
  (bind _outhits_2 (`KismetSystemLibrary.SphereTraceMulti` _returnvalue _returnvalue 150.0 "TraceTypeQuery3" false _array "ForDuration"))
  (bind _output_get (set `local.Targets` _outhits_2))
  (`KismetArrayLibrary.Array_Append` _output_get _outhits)
  (return _returnvalue_2 (`local.Targets`)))

(fn `UserConstructionScript`)