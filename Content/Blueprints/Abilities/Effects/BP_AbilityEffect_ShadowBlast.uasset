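; Shadow Blast ability effect that makes the casting top-down character unleash an area hit in front of itself.
; On activation it stops the caster, turns it toward its last movement input or current forward, and plays a montage.
; After a hit delay, it spawns Niagara VFX at a ground-traced forward point and shakes the camera.
; A sphere trace there applies reaction and damage through CombatInterface, then the effect finishes after its duration.
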(event `self.BP_Activate`
  (params (Caster :type "Character Object Reference"))
  (bind _hitloc (`self.HitLoc`))
  (bind _asbp_top_down_character (cast `/Game/Blueprints/Player/BP_TopDownCharacter` Caster))
  (bind _output_get (set `self.As BP Top Down Character` _asbp_top_down_character))
  (bind _charactermovement (`Character.CharacterMovement` _output_get))
  (`MovementComponent.StopMovementImmediately` _charactermovement)
  (`self.DefineDirection` _charactermovement)
  (`self.RotateToTarget` _charactermovement)
  (`Character.StopAnimMontage` _output_get null)
  (`Character.PlayAnimMontage` _output_get (`self.AnimToPlay`) 1.0 "None")
  (`KismetSystemLibrary.Delay` (`self.HitDelay`))
  (bind _output_get_2 (`self.GetHitLoc` _output_get))
  (bind _returnvalue (`NiagaraFunctionLibrary.SpawnSystemAtLocation` "/Game/VFX/ShadowBlast/NS_ShadowBlast.NS_ShadowBlast" _output_get_2))
  (bind _output_get_3 (set `self.VFX` _returnvalue))
  (`ActorComponent.Activate` _output_get_3 true)
  (`PlayerCameraManager.StartCameraShake` :`self` (`GameplayStatics.GetPlayerCameraManager` 0) :`ShakeClass` (`self.CameraShake`) :`Scale` 2.0)
  (bind (_outhits _returnvalue_2) (`KismetSystemLibrary.SphereTraceMulti` _hitloc _hitloc (`self.Radius`) "TraceTypeQuery3" false (`|MakeArray` (`self.As BP Top Down Character`) :!type "Actor Object Reference") "None" true (struct :`R` 1.0 :`A` 1.0) (struct :`G` 1.0 :`A` 1.0) 0.3))
  (if _returnvalue_2
    (for _array_element _outhits
      (bind (_bblockinghit _binitialoverlap _time _distance _location _impactpoint _normal _impactnormal _physmat _hitactor) (`GameplayStatics.BreakHitResult` _array_element))
      (bind _ascombat_interface (cast `CombatInterface` _hitactor))
      (`CombatInterface.OnSkillReaction` _ascombat_interface (`self.NPCReaction`))
      (`CombatInterface.Hit` _ascombat_interface null _impactpoint (* _impactnormal (`self.HitStrength`)) (`self.Damage`) true false null)))
  (`KismetSystemLibrary.Delay` (`self.EffectDuration`))
  (`self.OnEffectFinished` true))

(fn `DefineDirection`
  (params (Movement :type "PawnMovementComponent Object Reference"))
  (bind _returnvalue (`PawnMovementComponent.GetLastInputVector` Movement))
  (bind _as_bp_top_down_character (`self.As BP Top Down Character`))
  (set `self.CurrentRot` (`self.K2_GetActorRotation` _as_bp_top_down_character))
  (set `self.Dir` (`KismetMathLibrary.SelectVector` (`KismetMathLibrary.Normal` (`self.GetActorForwardVector` _as_bp_top_down_character)) _returnvalue (`KismetMathLibrary.Vector_IsNearlyZero` _returnvalue))))

(fn `GetHitLoc`
  (params (Actor :type "Actor Object Reference"))
  (returns (Output_Get :type "Vector Structure"))
  (bind _returnvalue (+ (`self.K2_GetActorLocation` Actor) (* (`KismetMathLibrary.Normal` (`self.GetActorForwardVector` Actor)) (`self.Offset`))))
  (set `self.HitLoc` _returnvalue)
  (bind (_outhit _returnvalue_2) (`KismetSystemLibrary.LineTraceSingle` (+ _returnvalue (0.0 0.0 150.0)) (- _returnvalue (0.0 0.0 500.0)) "TraceTypeQuery1" false (`|MakeArray` Actor) "None" true (struct :`R` 1.0 :`A` 1.0) (struct :`G` 1.0 :`A` 1.0) 0.2))
  (if _returnvalue_2
    (set `self.HitLoc` (`.Location` (`GameplayStatics.BreakHitResult` _outhit))))
  (return (`self.HitLoc`)))

(fn `RotateToTarget`
  (params (Movement :type "CharacterMovementComponent Object Reference"))
  (locals (TargetRot :type "Rotator Structure") (FinalRot :type "Rotator Structure"))
  (bind (_currentrot_roll _currentrot_pitch) (`KismetMathLibrary.BreakRotator` (`self.CurrentRot`)))
  (bind _returnvalue (`self.K2_GetActorLocation` (`self.As BP Top Down Character`)))
  (set `CharacterMovementComponent.bOrientRotationToMovement` false Movement)
  (bind _output_get (set `local.TargetRot` (`KismetMathLibrary.FindLookAtRotation` _returnvalue (+ _returnvalue (`self.Dir`)))))
  (bind _output_get_2 (set `local.FinalRot` (`KismetMathLibrary.MakeRotator` (.roll _output_get) _currentrot_pitch (.yaw _output_get))))
  (`self.K2_SetActorRotation` (`self.As BP Top Down Character`) _output_get_2 false)
  (set `CharacterMovementComponent.bOrientRotationToMovement` true Movement))

(fn `UserConstructionScript`)