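; Shadow Root ability effect that freezes enemies in a radius around the top-down character caster.
; On activation it plays the caster's montage and attached Niagara VFX, then after a delay sphere-traces pawns and freezes each unique EnemyInterface hit.
; A parallel branch signals effect completion early, waits FreezeDuration, then unfreezes those enemies and destroys the actor.
; The VFX position update, enemy reaction and HP-drain logic are disconnected.
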(event `self.BP_Activate`
  (params (Caster :type "Character Object Reference"))
  (bind _enemies (`self.Enemies`))
  (bind _returnvalue (`self.K2_GetActorLocation` (`self.As BP Top Down Character`)))
  (bind _asbp_top_down_character (cast `/Game/Blueprints/Player/BP_TopDownCharacter` Caster))
  (`Character.PlayAnimMontage` _asbp_top_down_character (`self.CharacterAnim Montage`) 1.0 "None")
  (bind _output_get (set `self.As BP Top Down Character` _asbp_top_down_character))
  (bind _returnvalue_2 (`NiagaraFunctionLibrary.SpawnSystemAttached` "/Game/VFX/ShadowRoot/NS_ShadowRoot.NS_ShadowRoot" (`Actor.RootComponent` _output_get) "None" (0.0 0.0 0.0) (struct) "SnapToTarget" true))
  (set `self.VFX` _returnvalue_2)
  (`|ExecutionSequence`
    (:`then_0`
      (`KismetSystemLibrary.Delay` 1.0)
      (set `self.Enemies` (`|MakeArray`))
      (bind (_outhits _returnvalue_3) (`KismetSystemLibrary.SphereTraceMultiForObjects` _returnvalue _returnvalue (`self.Radius`) (`|MakeArray` "ObjectTypeQuery3" :!type "EObjectTypeQuery Enum") false (`|MakeArray` (`self.As BP Top Down Character`) :!type "Actor Object Reference")))
      (if _returnvalue_3
        (for _array_element _outhits
          (bind (_bblockinghit _binitialoverlap _time _distance _location _impactpoint _normal _impactnormal _physmat _hitactor) (`GameplayStatics.BreakHitResult` _array_element))
          (bind _asenemy_interface (cast `EnemyInterface` _hitactor))
          (if (not (`KismetArrayLibrary.Array_Contains` _enemies _hitactor))
            (`EnemyInterface.Freeze` _asenemy_interface true)
            (`KismetArrayLibrary.Array_Add` _enemies _hitactor)
            (`KismetArrayLibrary.Array_Add` (`self.Positions`) (`self.K2_GetActorLocation` _hitactor))))))
    (:`then_1`
      (`KismetSystemLibrary.Delay` 0.1)
      (`self.OnEffectFinished` false)
      (`KismetSystemLibrary.Delay` (`self.FreezeDuration`))
      (for _array_element_2 (`self.Enemies`)
        (bind _asenemy_interface_2 (cast `EnemyInterface` _array_element_2))
        (`EnemyInterface.Freeze` _asenemy_interface_2 false))
      (`self.K2_DestroyActor`))))

(event `self.ReceiveTick`
  (params (DeltaSeconds :type "Float (single-precision)")))

(fn `UserConstructionScript`)