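; Roar of Flames ability effect that breathes a cone of fire from the casting top-down character, damaging what it hits.
; Activation attaches a Niagara system to the caster, with Tick keeping its Position parameter on the head socket.
; A debug-drawn cone trace from the head follows mesh facing, offset 90 degrees in yaw.
; After a short delay, hits receive enemy reactions and damage through interfaces, then the effect signals completion.
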(event `self.BP_Activate`
  (params (Caster :type "Character Object Reference"))
  (bind _mesh (`Character.Mesh` (`self.As BP Top Down Character`)))
  (bind (_returnvalue_roll _returnvalue_pitch _returnvalue_yaw) (`KismetMathLibrary.BreakRotator` (`SceneComponent.GetSocketRotation` _mesh "None")))
  (bind _asbp_top_down_character (cast `/Game/Blueprints/BP_TopDownCharacter` Caster))
  (bind _output_get (set `self.As BP Top Down Character` _asbp_top_down_character))
  (bind _returnvalue (`NiagaraFunctionLibrary.SpawnSystemAttached` "/Game/VFX/RoarOfFlames/NS_RoarOfFlames.NS_RoarOfFlames" (`Actor.RootComponent` _output_get) "None" (0.0 0.0 0.0) (struct) "SnapToTarget" true))
  (set `self.VFX` _returnvalue)
  (bind _returnvalue_location (`KismetMathLibrary.BreakTransform` (`SceneComponent.GetSocketTransform` (`Character.Mesh` _output_get) "head" "RTS_Actor")))
  (`NiagaraComponent.SetVariableVec3` _returnvalue "Position" _returnvalue_location)
  (`ActorComponent.Activate` _returnvalue true)
  (bind (_outhits _returnvalue_2) (`RPGFunctionsLibrary.ConeTraceMulti` (`SceneComponent.GetSocketLocation` _mesh "head") (`KismetMathLibrary.MakeRotator` _returnvalue_roll _returnvalue_pitch (+ _returnvalue_yaw 90.0)) (`self.Radius`) 22.5 "TraceTypeQuery3" false (`|MakeArray` (`self.As BP Top Down Character`) :!type "Actor Object Reference") "ForDuration" (struct :`R` 0.412908 :`G` 1.0 :`B` 0.045183 :`A` 1.0) (struct :`R` 1.0 :`B` 0.114695 :`A` 1.0) 5.0))
  (`KismetSystemLibrary.Delay` 0.2)
  (if _returnvalue_2
    (for _array_element _outhits
      (bind (_bblockinghit _binitialoverlap _time _distance _location _impactpoint _normal _impactnormal _physmat _hitactor) (`GameplayStatics.BreakHitResult` _array_element))
      (bind _asenemy_interface (cast `EnemyInterface` _hitactor))
      (`EnemyInterface.OnHit` _asenemy_interface null _impactpoint (0.0 0.0 0.0))
      (`EnemyInterface.OnSkillReaction` _asenemy_interface (`self.NPCReaction`))
      (bind _asdamageable_interface (cast `DamageableInterface` _hitactor))
      (`DamageableInterface.Damage` _asdamageable_interface (`self.Damage`))))
  (`KismetSystemLibrary.Delay` 1.0)
  (`self.OnEffectFinished`))

(event `self.ReceiveTick`
  (params (DeltaSeconds :type "Float (single-precision)"))
  (bind _returnvalue_location (`KismetMathLibrary.BreakTransform` (`SceneComponent.GetSocketTransform` (`Character.Mesh` (`self.As BP Top Down Character`)) "head" "RTS_Actor")))
  (if (and (`KismetSystemLibrary.IsValid` (`self.As BP Top Down Character`)) (`KismetSystemLibrary.IsValid` (`self.VFX`)))
    (`NiagaraComponent.SetVariableVec3` (`self.VFX`) "Position" _returnvalue_location)))

(fn `UserConstructionScript`)