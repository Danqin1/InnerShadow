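; Shadow Cut ability effect that turns the casting RPG character toward its last movement input and plays an attack animation.
; On activation it snaps the yaw to that direction, switches movement to Flying, replaces any current montage with its own and resets the combat component's attack.
; After the effect duration it signals that the effect finished and restores Walking mode.
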(event `self.BP_Activate`
  (params (Caster :type "Character Object Reference"))
  (bind (_currentrot_roll _currentrot_pitch) (`KismetMathLibrary.BreakRotator` (`self.CurrentRot`)))
  (bind _asrpgcharacter (cast `RPGCharacter` Caster)
    (:`then`
      (bind _charactermovement (`Character.CharacterMovement` _asrpgcharacter))
      (set `CharacterMovementComponent.bOrientRotationToMovement` false _charactermovement)
      (set `self.Direction` (`PawnMovementComponent.GetLastInputVector` _charactermovement))
      (bind _returnvalue (`self.K2_GetActorLocation` _asrpgcharacter))
      (set `self.Start` _returnvalue)
      (set `self.End` (+ _returnvalue (* (`self.Direction`) 1000.0)))
      (set `self.CurrentRot` (`self.K2_GetActorRotation` _asrpgcharacter))
      (bind _output_get (set `self.TargetRot` (`KismetMathLibrary.FindLookAtRotation` (`self.Start`) (`self.End`))))
      (bind _output_get_2 (set `self.FinalRot` (`KismetMathLibrary.MakeRotator` (.roll _output_get) _currentrot_pitch (.yaw _output_get))))
      (`self.K2_SetActorRotation` _asrpgcharacter _output_get_2 false)
      (`CharacterMovementComponent.SetMovementMode` _charactermovement "MOVE_Flying" 0)
      (set `CharacterMovementComponent.bOrientRotationToMovement` true _charactermovement)
      (`Character.StopAnimMontage` _asrpgcharacter null)
      (`Character.PlayAnimMontage` _asrpgcharacter (`self.Anim`) 1.0 "None")
      (`CombatComponent.ResetAttack` (`RPGCharacter.CombatComponent` _asrpgcharacter))
      (`KismetSystemLibrary.Delay` (`self.EffectDuration`))
      (`self.OnEffectFinished` true)
      (`CharacterMovementComponent.SetMovementMode` _charactermovement "MOVE_Walking" 0))
    (:`CastFailed`
      (`KismetSystemLibrary.PrintString` "Cast to character failed" true true (struct :`R` 1.0 :`B` 0.036312 :`A` 1.0)))))

(fn `UserConstructionScript`)